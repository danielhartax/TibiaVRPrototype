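; Projectile spell that homes in on the enemy under the player's crosshair, or flies straight along the camera view when none is targeted.
; On BeginPlay, SetTargetWithDelay line-traces from the camera to pick that mode immediately (its delay and target-actor spawn are disconnected), and the projectile expires after a fixed lifetime.
; Overlapping an enemy applies dice-rolled damage; any overlap except the player's floating hands plays a sound and destroys it.
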(event OnComponentBeginOverlap(SphereCollider)
  (params (OverlappedComponent :type Primitive%20Component%20Object%20Reference) (OtherActor :type Actor%20Object%20Reference) (OtherComp :type Primitive%20Component%20Object%20Reference) (OtherBodyIndex :type Integer) (bFromSweep :type Boolean) (SweepResult :type Hit%20Result%20Structure%20%28by%20ref%29))
  (if (Class|GameplayStatics|ObjectIsA OtherActor "/Game/Blueprints/Monsters/BP_Enemy.BP_Enemy_C")
    (CallFunction|RollDiceandApplyDamage (Variables|Default|GetDamageDice) (Variables|Default|GetDiceQuantity) OtherActor (Components|GetOwner))
    (CallFunction|PlaySoundEffectonSpawn :!label _label)
    (Actor|DestroyActor)
    (elif (not (or (Class|GameplayStatics|ObjectIsA OtherActor "/Game/Blueprints/PlayerFloatingHands/BP_PlayerFloatingHands.BP_PlayerFloatingHands_C") (Class|GameplayStatics|ObjectIsA OtherActor "/Game/Blueprints/Monsters/BP_Enemy.BP_Enemy_C")))
      (goto _label))))

(event EventBeginPlay
  (|CallParentFunction)
  (Utilities|SetTargetwithDelay (Variables|Default|GetDelay))
  (Utilities|FlowControl|Delay 5.0)
  (Actor|DestroyActor))

(event Collision|EventActorBeginOverlap
  (params (OtherActor :type Actor%20Object%20Reference)))

(event EventTick
  (params (DeltaSeconds :type Float%20%28single-precision%29)))

(fn ConstructionScript)