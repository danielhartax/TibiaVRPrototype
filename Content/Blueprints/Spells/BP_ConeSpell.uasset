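; BP_ConeSpell is a short-lived cone-shaped spell actor that damages monsters entering its collider.
; On BeginPlay it waits for a set duration, then destroys itself.
; When ConeCollider begins overlapping a BP_Monster, it rolls the configured damage dice and applies the damage, crediting the spell's owner as causer.
; CheckConeCollision is an empty stub, so hit detection relies solely on the overlap event.
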(event OnComponentBeginOverlap(ConeCollider)
  (params (OverlappedComponent :type Primitive%20Component%20Object%20Reference) (OtherActor :type Actor%20Object%20Reference) (OtherComp :type Primitive%20Component%20Object%20Reference) (OtherBodyIndex :type Integer) (bFromSweep :type Boolean) (SweepResult :type Hit%20Result%20Structure%20%28by%20ref%29))
  (if (Class|GameplayStatics|ObjectIsA OtherActor "/Game/Blueprints/Monsters/BP_Monster.BP_Monster_C")
    (CallFunction|RollDiceandApplyDamage (Variables|Default|GetDamageDice) (Variables|Default|GetDiceQuantity) OtherActor (Components|GetOwner))))

(event EventBeginPlay
  (|CallParentFunction)
  (Utilities|FlowControl|Delay (Variables|Default|GetDurantion))
  (Actor|DestroyActor))

(event Collision|EventActorBeginOverlap
  (params (OtherActor :type Actor%20Object%20Reference))
  (|CallParentFunction OtherActor) ; This node is disabled and will not be called.\nDrag off pins to build functionality.
)

(event EventTick
  (params (DeltaSeconds :type Float%20%28single-precision%29))
  (|CallParentFunction DeltaSeconds) ; This node is disabled and will not be called.\nDrag off pins to build functionality.
)

(fn ConstructionScript
  (|CallParentFunction))

(fn CheckConeCollision)