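; VR player pawn with floating hands that handles locomotion, grabbing, weapon skills and health.
; Grip and trigger axes animate the hands; movement follows left-hand yaw, with delay-gated snap turning.
; Grabs take the slotted actor or box-trace for BPI_GrabbableActor, messaging it on grab and drop; the right secondary button casts held-weapon skills.
; Inventory tracks headset position and yaw at half height, and death teleports to the BeginPlay checkpoint, restoring HP.
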(event EventBeginPlay
  (Class|HeadMountedDisplayFunctionLibrary|SetTrackingOrigin "Floor")
  (Variables|Default|SetCheckPoint (Transformation|GetActorLocation))
  (Variables|Default|SetMaxHP (Variables|Default|GetHP)))

(event Collision|EventActorBeginOverlap
  (params (OtherActor :type Actor%20Object%20Reference)))

(event EventTick
  (params (DeltaSeconds :type Float%20%28single-precision%29))
  (CallFunction|UpdateInventoryRotation))

(event Game|Damage|EventAnyDamage
  (params (Damage :type Float%20%28single-precision%29) (DamageType :type Damage%20Type%20Object%20Reference) (InstigatedBy :type Controller%20Object%20Reference) (DamageCauser :type Actor%20Object%20Reference))
  ;[1 1 1] recebe dano
  (bind _output_get (Variables|Default|SetHP (Math|Float|Truncate (- (Variables|Default|GetHP) Damage))))
  (if (<= _output_get 0)
    (CallFunction|KillPlayer)))

(event Input|ActionEvents|InputActionGrabLeft
  (params (Key :type Key%20Structure :default "None"))
  ;[1 1 1] Grab e Drop
  (:Pressed
    (bind _grabbedactor (CallFunction|ExecuteGrab (Variables|Default|GetMotionController_Left)))
    (Variables|Default|SetGrabbedActor_Left _grabbedactor))
  (:Released
    (bind _releasedactor (CallFunction|ExecuteDrop (Variables|Default|GetGrabbedActor_Left) (Variables|Default|GetMotionController_Left)))
    (Variables|Default|SetGrabbedActor_Left _releasedactor)
    (Variables|Default|SetSlotedActor 0)))

(event Input|ActionEvents|InputActionGrabRight
  (params (Key :type Key%20Structure :default "None"))
  ;[1 1 1] Grab e Drop
  (:Pressed
    (bind _grabbedactor (CallFunction|ExecuteGrab (Variables|Default|GetMotionController_Right)))
    (Variables|Default|SetGrabbedActor_Right _grabbedactor))
  (:Released
    (CallFunction|ExecuteDrop (Variables|Default|GetGrabbedActor_Right) (Variables|Default|GetMotionController_Right))
    (Variables|Default|SetGrabbedActor_Right 0)
    (Variables|Default|SetSlotedActor 0)))

(event Input|ActionEvents|InputActionSecondaryButtonRight
  (params (Key :type Key%20Structure :default "None"))
  (bind _grabbedactor_right (Variables|Default|GetGrabbedActor_Right))
  ;[1 1 1] Cast Skill
  (:Pressed
    (Utilities|IsValid _grabbedactor_right
      (:Is%20Valid
        (bind _asbp_weapon (Utilities|Casting|CastToBP_Weapon _grabbedactor_right))
        (Class|BPIClassSkills|CastSkill(Message) _asbp_weapon)))))

(event Input|AxisEvents|InputAxisGripAxis_Left
  (params (AxisValue :type Float%20%28single-precision%29))
  ;[1 1 1] Animacao da mão abrindo e fechando com o grip e trigger
  (bind _asabp_vrhand (Utilities|Casting|CastToABP_VRHand (Components|SkeletalMesh|GetAnimInstance (Variables|Default|GetHandMesh_Left))))
  (Variables|/Game/Characters/Animations/PlayerFloatingHands/ABP_VRHand.ABP_VRHand_C|SetGrip _asabp_vrhand AxisValue))

(event Input|AxisEvents|InputAxisGripAxis_Right
  (params (AxisValue :type Float%20%28single-precision%29))
  ;[1 1 1] Animacao da mão abrindo e fechando com o grip e trigger
  (bind _asabp_vrhand (Utilities|Casting|CastToABP_VRHand (Components|SkeletalMesh|GetAnimInstance (Variables|Default|GetHandMesh_Right))))
  (Variables|/Game/Characters/Animations/PlayerFloatingHands/ABP_VRHand.ABP_VRHand_C|SetGrip _asabp_vrhand AxisValue))

(event Input|AxisEvents|InputAxisMoveForward
  (params (AxisValue :type Float%20%28single-precision%29))
  ;[1 1 1] Movement
  (Pawn|Input|AddMovementInput (Math|Vector|GetForwardVector (Math|Rotator|MakeRotator 0.0 0.0 (.yaw (Transformation|GetWorldRotation (Variables|Default|GetHandMesh_Left))))) AxisValue false))

(event Input|AxisEvents|InputAxisMoveSide
  (params (AxisValue :type Float%20%28single-precision%29))
  ;[1 1 1] Movement
  (Pawn|Input|AddMovementInput (Math|Vector|GetRightVector (Math|Rotator|MakeRotator 0.0 0.0 (.yaw (Transformation|GetWorldRotation (Variables|Default|GetHandMesh_Left))))) AxisValue false))

(event Input|AxisEvents|InputAxisSnapTurn
  (params (AxisValue :type Float%20%28single-precision%29))
  (bind _snapturninputdeadzone (Variables|Default|GetSnapTurnInputDeadZone))
  ;[1 1 1] SnapTurn
  (if (not (Variables|Default|GetIsSnapTurnActive))
    (if (>= AxisValue _snapturninputdeadzone)
      (Pawn|Input|AddControllerYawInput (Variables|Default|GetSnapTurnIncrement)) ; Vira pra direita
      (Variables|Default|SetIsSnapTurnActive true :!label _label)
      (Utilities|FlowControl|Delay (Variables|Default|GetDelayToSnapTurnAgain))
      (Variables|Default|SetIsSnapTurnActive false)
      (elif (<= AxisValue (* _snapturninputdeadzone -1.0))
        (Pawn|Input|AddControllerYawInput (* (Variables|Default|GetSnapTurnIncrement) -1.0)) ; vira pra esquerda
        (goto _label)))))

(event Input|AxisEvents|InputAxisTriggerAxis_Left
  (params (AxisValue :type Float%20%28single-precision%29))
  ;[1 1 1] Animacao da mão abrindo e fechando com o grip e trigger
  (bind _asabp_vrhand (Utilities|Casting|CastToABP_VRHand (Components|SkeletalMesh|GetAnimInstance (Variables|Default|GetHandMesh_Left))))
  (Variables|/Game/Characters/Animations/PlayerFloatingHands/ABP_VRHand.ABP_VRHand_C|SetTrigger _asabp_vrhand AxisValue))

(event Input|AxisEvents|InputAxisTriggerAxis_Right
  (params (AxisValue :type Float%20%28single-precision%29))
  ;[1 1 1] Animacao da mão abrindo e fechando com o grip e trigger
  (bind _asabp_vrhand (Utilities|Casting|CastToABP_VRHand (Components|SkeletalMesh|GetAnimInstance (Variables|Default|GetHandMesh_Right))))
  (Variables|/Game/Characters/Animations/PlayerFloatingHands/ABP_VRHand.ABP_VRHand_C|SetTrigger _asabp_vrhand AxisValue))

(fn ConstructionScript)

(fn FindNearestObjecttoGrab
  (params (MotionController :type Scene%20Component%20Object%20Reference))
  (bind _returnvalue (Transformation|GetWorldLocation MotionController))
  (bind _slotedactor (Variables|Default|GetSlotedActor)
    (:then
      (Transformation|SetActorLocation _slotedactor _returnvalue false false)
      (Transformation|SetActorRotation _slotedactor (Transformation|GetWorldRotation MotionController))
      (return _slotedactor))
    (:else
      (bind _outhit (Collision|BoxTraceByChannel _returnvalue (+ _returnvalue (* (Math|Vector|GetForwardVector MotionController) (Variables|Default|GetBoxTraceLength))) "0, 0, 0" "0, 0, 0" "TraceTypeQuery1" false 0 "None"))
      (if (Utilities|DoesObjectImplementInterface (.HitActor (Collision|BreakHitResult _outhit)) "/Game/Blueprints/Weapons/BPI_GrabbableActor.BPI_GrabbableActor_C")
        (return (.HitActor (Collision|BreakHitResult _outhit)))
        (else
          (return 0))))))

(fn ExecuteGrab
  (params (MotionController :type Scene%20Component%20Object%20Reference))
  (bind _availablegrabbableactor (CallFunction|FindNearestObjecttoGrab MotionController))
  (Utilities|IsValid _availablegrabbableactor
    (:Is%20Valid
      (Class|BPIGrabbableActor|Grab(Message) _availablegrabbableactor MotionController)
      (return _availablegrabbableactor))))

(fn ExecuteDrop
  (params (GrabbedActor :type Actor%20Object%20Reference) (Grabber :type Scene%20Component%20Object%20Reference))
  (Class|BPIGrabbableActor|Drop(Message) GrabbedActor Grabber)
  (return 0))

(fn UpdateInventoryRotation
  (bind _inventory (Variables|Default|GetInventory))
  (bind _camera (Variables|Default|GetCamera))
  (bind _relativelocation (Variables|/Script/Engine.SceneComponent|GetRelativeLocation _camera))
  (Transformation|SetRelativeLocation _inventory (Math|Vector|MakeVector (.x _relativelocation) (.y _relativelocation) (/ (.z _relativelocation) 2.0)) false true)
  (Transformation|SetRelativeRotation _inventory (Math|Rotator|MakeRotator 0.0 0.0 (.yaw (Variables|/Script/Engine.SceneComponent|GetRelativeRotation _camera))) false false))

(fn KillPlayer
  (Transformation|Teleport (Variables|Default|GetCheckPoint) "0, 0, 0")
  (Variables|Default|SetHP (Variables|Default|GetMaxHP)))

(fn Heal
  (params (HealValue :type Integer))
  (if (> (+ HealValue (Variables|Default|GetHP)) (Variables|Default|GetMaxHP))
    (Variables|Default|SetHP (Variables|Default|GetMaxHP))
    (else
      (Variables|Default|SetHP 0))))