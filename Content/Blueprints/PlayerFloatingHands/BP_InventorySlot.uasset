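; Inventory slot collision component, filed with the floating-hands player, that holds one BP_GrabbableActor at a time.
; Its overlap events track the first grabbable to enter while the slot is empty, and clear it when that actor leaves.
; Each Tick, if the tracked actor has no valid GrabberOne, it attaches to the slot, snapping location and rotation while keeping world scale.
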(event Custom|BeginOverlap
  (params (OverlappedComponent :type Primitive%20Component%20Object%20Reference) (OtherActor :type Actor%20Object%20Reference) (OtherComp :type Primitive%20Component%20Object%20Reference) (OtherBodyIndex :type Integer) (bFromSweep :type Boolean) (SweepResult :type Hit%20Result%20Structure%20%28by%20ref%29))
  (Variables|Default|GetGrabbabeActor
    (:then)
    (:else
      (bind _asbp_grabbable_actor (Utilities|Casting|CastToBP_GrabbableActor OtherActor))
      (Variables|Default|SetGrabbabeActor _asbp_grabbable_actor))))

(event Custom|EndOverlap
  (params (OverlappedComponent :type Primitive%20Component%20Object%20Reference) (OtherActor :type Actor%20Object%20Reference) (OtherComp :type Primitive%20Component%20Object%20Reference) (OtherBodyIndex :type Integer))
  (if (== OtherActor (Variables|Default|GetGrabbabeActor))
    (Variables|Default|SetGrabbabeActor 0)))

(event EventBeginPlay
  (Collision|BindEventtoOnComponentBeginOverlap (delegate Custom|BeginOverlap))
  (Collision|BindEventtoOnComponentEndOverlap (delegate Custom|EndOverlap)))

(event EventTick
  (params (DeltaSeconds :type Float%20%28single-precision%29))
  (bind _grabbabeactor (Variables|Default|GetGrabbabeActor)
    (:then
      (Variables|/Game/Blueprints/Weapons/BP_GrabbableActor.BP_GrabbableActor_C|GetGrabberOne _grabbabeactor
        (:then)
        (:else
          (Transformation|AttachComponentToComponent _grabbabeactor self "None" "SnapToTarget" "SnapToTarget" "KeepWorld" true))))
    (:else)))