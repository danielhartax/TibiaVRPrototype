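; BP_Enemy is a melee enemy, apparently a goblin, that detects and attacks the floating-hands player.
; Pawn sensing sets a seen-player flag in the AI Blackboard, which also receives a zero-vector initial position on BeginPlay.
; AttackPlayer sphere-traces forward, plays a slash montage on a player hit and applies dice-rolled damage, leaving persistent debug drawing.
; Construction makes armor pieces follow the body mesh's pose and snaps the weapon to the hand socket.
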(event OnSeePawn(PawnSensing)
  (params (Pawn :type Pawn%20Object%20Reference))
  (Utilities|Casting|CastToBP_PlayerFloatingHands Pawn)
  (AI|Components|Blackboard|SetValueasBool (Variables|Default|GetAIBlackboard) (Utilities|Name|MakeLiteralName "HasSeenPlayer") true))

(event Custom|AttackPlayer
  (bind _returnvalue (Transformation|GetActorLocation))
  (bind (_outhit _returnvalue_2) (Collision|SphereTraceForObjects _returnvalue (+ _returnvalue (* (Math|Vector|GetForwardVector (Transformation|GetActorRotation)) 6e+01)) 2e+02 (Utilities|Array|MakeArray "ObjectTypeQuery7") false 0 "Persistent"))
  (if _returnvalue_2
    (bind _asbp_player_floating_hands (Utilities|Casting|CastToBP_PlayerFloatingHands (.HitActor (Collision|BreakHitResult _outhit))))
    (Animation|PlayAnimMontage "/Game/Blueprints/Monsters/Animations/Anim_Goblin_body_attack_slash_Montage.Anim_Goblin_body_attack_slash_Montage" 1.0 "None")
    (CallFunction|RollDiceandApplyDamage (Variables|Default|GetDamageDice) (Variables|Default|GetDiceQuantity) _asbp_player_floating_hands self)))

(event EventBeginPlay
  (bind _output_get (Variables|Default|SetAIBlackboard (AI|GetBlackboard (AI|GetAIController self))))
  (AI|Components|Blackboard|SetValueasVector _output_get (Utilities|Name|MakeLiteralName "InitialPosition") "0, 0, 0"))

(event Collision|EventActorBeginOverlap
  (params (OtherActor :type Actor%20Object%20Reference)))

(event EventTick
  (params (DeltaSeconds :type Float%20%28single-precision%29)))

(fn ConstructionScript
  (Components|SkinnedMesh|SetLeaderPoseComponent (Variables|Default|GetHelmet) (Variables|Character|GetMesh) true true)
  (Transformation|AttachComponentToComponent (Variables|Default|GetWeapon) (Variables|Character|GetMesh) "hand" "SnapToTarget" "SnapToTarget" "KeepWorld" false))