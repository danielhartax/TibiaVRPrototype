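; BP_Monster is a monster actor with hit points that is destroyed when its HP runs out.
; On BeginPlay it binds to its own OnTakeAnyDamage event, which truncates incoming damage to an integer and passes it to TakeDamage.
; TakeDamage subtracts that value from HP and calls Kill at zero or below, which simply destroys the actor.
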(event Custom|OnTakeAnyDamage_Event
  (params (DamagedActor :type Actor%20Object%20Reference) (Damage :type Float%20%28single-precision%29) (DamageType :type Damage%20Type%20Object%20Reference) (InstigatedBy :type Controller%20Object%20Reference) (DamageCauser :type Actor%20Object%20Reference))
  (CallFunction|TakeDamage (Math|Float|Truncate Damage)))

(event EventBeginPlay
  (EventDispatchers|BindEventtoOnTakeAnyDamage (delegate Custom|OnTakeAnyDamage_Event)))

(event Collision|EventActorBeginOverlap
  (params (OtherActor :type Actor%20Object%20Reference)))

(event EventTick
  (params (DeltaSeconds :type Float%20%28single-precision%29)))

(fn ConstructionScript)

(fn TakeDamage
  (params (DamageValue :type Integer))
  (Variables|Default|SetHP (- (Variables|Default|GetHP) DamageValue))
  (if (<= (Variables|Default|GetHP) 0)
    (CallFunction|Kill)))

(fn Kill
  (Actor|DestroyActor))