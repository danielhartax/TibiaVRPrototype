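; BP_Weapon is a weapon Blueprint that damages BP_Enemy actors when its mesh overlaps them, likely serving as a base class.
; Hits roll dice for damage, halved for two-handed weapons not held two-handed, then play a sound and stay locked until an overlap ends.
; Skill casting and special attacks have delay-based cooldowns around CanCast, ExecuteSkill and ExecuteSpecialAttack, which are debug-print placeholders here.
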(event OnComponentBeginOverlap(StaticMesh)
  (params (OverlappedComponent :type Primitive%20Component%20Object%20Reference) (OtherActor :type Actor%20Object%20Reference) (OtherComp :type Primitive%20Component%20Object%20Reference) (OtherBodyIndex :type Integer) (bFromSweep :type Boolean) (SweepResult :type Hit%20Result%20Structure%20%28by%20ref%29))
  ;[1 1 1] Damage
  (if (Variables|Default|GetCanHit)
    (if (Class|GameplayStatics|ObjectIsA OtherActor "/Game/Blueprints/Monsters/BP_Enemy.BP_Enemy_C")
      (if (Variables|Default|GetIsTwoHanded)
        (if (Variables|Default|GetIsHeldWithTwoHands)
          (bind _result (CallFunction|RollDice (Variables|Default|GetDamageDice) (Variables|Default|GetDiceQuantity) :!label _label))
          (Variables|Default|SetDamageResult _result)
          (else
            (bind _result_2 (CallFunction|RollDice (Variables|Default|GetDamageDice) (Variables|Default|GetDiceQuantity)))
            (Variables|Default|SetDamageResult (/ _result_2 2))))
        (else
          (goto _label)))
      (Game|Damage|ApplyDamage OtherActor (Math|Conversions|ToFloat(Integer) (Variables|Default|GetDamageResult)) 0 0)
      (Audio|PlaySoundatLocation (Variables|Default|GetDamageSound) (Transformation|GetWorldLocation (Variables|Default|GetStaticMesh)) "0, 0, 0" 1.0 1.0 0.0 0 0 0 0)
      (Variables|Default|SetCanHit false))))

(event OnComponentEndOverlap(StaticMesh)
  (params (OverlappedComponent :type Primitive%20Component%20Object%20Reference) (OtherActor :type Actor%20Object%20Reference) (OtherComp :type Primitive%20Component%20Object%20Reference) (OtherBodyIndex :type Integer))
  ;[1 1 1] Damage
  (Variables|Default|SetCanHit true))

(event EventBeginPlay
  (|CallParentFunction)
  (bind _asbp_player_floating_hands (Utilities|Casting|CastToBP_PlayerFloatingHands (Game|GetPlayerCharacter 0)))
  (Variables|Default|SetPlayerClass _asbp_player_floating_hands))

(event Collision|EventActorBeginOverlap
  (params (OtherActor :type Actor%20Object%20Reference))
  (|CallParentFunction OtherActor) ; This node is disabled and will not be called.\nDrag off pins to build functionality.
)

(event EventTick
  (params (DeltaSeconds :type Float%20%28single-precision%29))
  (|CallParentFunction DeltaSeconds) ; This node is disabled and will not be called.\nDrag off pins to build functionality.
)

(event EventCastSkill
  ;[1 1 1] Cast skill
  (if (not (Variables|Default|GetIsRecharging))
    (Variables|Default|SetIsRecharging true)
    (if (CallFunction|CanCast)
      (CallFunction|ExecuteSkill)
      (Utilities|FlowControl|Delay (Variables|Default|GetCoolDown))
      (Variables|Default|SetIsRecharging false))))

(event EventSpecialAttack
  (CallFunction|ExecuteSpecialAttack)
  (Variables|Default|SetCanUseSpecialAttack false)
  (Utilities|FlowControl|Delay 2.0)
  (Variables|Default|SetCanUseSpecialAttack true))

(fn ConstructionScript
  (|CallParentFunction))

(fn CanCast
  (Development|PrintString "ENTROU NO CAN CAST DO PAI" true true "(R=1.000000,G=0.891643,B=0.000000,A=1.000000)")
  (return true))

(fn ExecuteSkill
  (Development|PrintString "Executou a magia" true true "(R=1.000000,G=0.420393,B=0.208745,A=1.000000)")
  (return))

(fn ExecuteSpecialAttack
  (Development|PrintString "USOU O SPECIAL ATTACK"))