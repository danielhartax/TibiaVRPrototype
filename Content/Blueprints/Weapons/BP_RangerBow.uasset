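; Two-handed grabbable bow for the floating-hands player: the first grabber holds it, and a second one at the string spawns and nocks an arrow.
; While drawn, Tick projects the pulling hand onto the bow's axis to move the string and measure charge.
; Releasing the string plays a snap-back timeline that launches the arrow at charge-scaled strength.
; A near-full draw enables the skill that enchants the arrow.
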(event OnComponentBeginOverlap(StringCollision)
  (params (OverlappedComponent :type Primitive%20Component%20Object%20Reference) (OtherActor :type Actor%20Object%20Reference) (OtherComp :type Primitive%20Component%20Object%20Reference) (OtherBodyIndex :type Integer) (bFromSweep :type Boolean) (SweepResult :type Hit%20Result%20Structure%20%28by%20ref%29))
  (if (Class|GameplayStatics|ObjectIsA OtherActor "/Game/Blueprints/PlayerFloatingHands/BP_PlayerFloatingHands.BP_PlayerFloatingHands_C")
    (Variables|Default|SetIsTryingToPullTheString true)))

(event OnComponentEndOverlap(StringCollision)
  (params (OverlappedComponent :type Primitive%20Component%20Object%20Reference) (OtherActor :type Actor%20Object%20Reference) (OtherComp :type Primitive%20Component%20Object%20Reference) (OtherBodyIndex :type Integer))
  (if (Class|GameplayStatics|ObjectIsA OtherActor "/Game/Blueprints/PlayerFloatingHands/BP_PlayerFloatingHands.BP_PlayerFloatingHands_C")
    (Variables|Default|SetIsTryingToPullTheString false)))

(event Custom|Shoot
  (Components|Timeline|SetPlayRate (Variables|Default|GetSnapBack) (/ 1.0 0.05))
  (bind _newtrack_0 (Timeline|SnapBack PlayFromStart)
    (:Update
      (Transformation|SetRelativeLocation (Variables|Default|GetString) (Math|Vector|Lerp(Vector) (Variables|Default|GetStringRelativeLocation) (Variables|/Script/Engine.SceneComponent|GetRelativeLocation (Variables|Default|GetStringCollision)) _newtrack_0) false false)
      (if (> _newtrack_0 0.8)
        (bind _arrow (Variables|Default|GetArrow)
          (:then
            (Transformation|DetachFromActor _arrow "KeepWorld" "KeepWorld" "KeepWorld")
            (Default|Shoot _arrow (Math|Float|MapRangeClamped (Variables|Default|GetStringCharge) 0.0 6e+01 0.0 2e+03)))
          (:else))))
    (:Finished
      (Utilities|FlowControl|Delay 0.1)
      (CallFunction|HideString))))

(event EventBeginPlay
  (|CallParentFunction))

(event Collision|EventActorBeginOverlap
  (params (OtherActor :type Actor%20Object%20Reference))
  (|CallParentFunction OtherActor) ; This node is disabled and will not be called.\nDrag off pins to build functionality.
)

(event EventTick
  (params (DeltaSeconds :type Float%20%28single-precision%29))
  (CallFunction|StringStrech))

(fn ConstructionScript
  (|CallParentFunction)
  (CallFunction|HideString))

(fn ExecuteGrab
  (params (InputPin :type Scene%20Component%20Object%20Reference))
  (Variables|Default|GetGrabberOne
    (:then
      (if (Variables|Default|GetIsTryingToPullTheString)
        (Variables|Default|SetGrabberTwo InputPin)
        (Actor|Tick|SetActorTickEnabled true)
        (CallFunction|ShowString)
        (bind _returnvalue (Game|SpawnActorfromClass "/Game/Blueprints/Weapons/BP_RangerArrow.BP_RangerArrow_C" (Math|Transform|MakeTransform "0, 0, 0") "AlwaysSpawn" "MultiplyWithRoot" 0 0))
        (bind _output_get (Variables|Default|SetArrow _returnvalue))
        (Transformation|AttachComponentToComponent _output_get (Variables|Default|GetString) "None" "SnapToTarget" "SnapToTarget" "KeepWorld" true)))
    (:else
      (bind _output_get_2 (Variables|Default|SetGrabberOne InputPin))
      (Physics|SetSimulatePhysics (Variables|Default|GetStaticMesh) false)
      (Transformation|AttachComponentToComponent (Components|GetChildComponent _output_get_2 0) "bow" "SnapToTarget" "SnapToTarget" "KeepWorld" true))))

(fn ExecuteRelease
  (params (Grabber :type Scene%20Component%20Object%20Reference))
  (if (== Grabber (Variables|Default|GetGrabberOne))
    (Physics|SetSimulatePhysics (Variables|Default|GetStaticMesh) true)
    (Transformation|DetachFromActor "KeepRelative" "KeepWorld" "KeepWorld")
    (Variables|Default|SetGrabberOne 0)
    (Variables|Default|SetGrabberTwo 0)
    (Actor|Tick|SetActorTickEnabled false)
    (else
      (Variables|Default|SetGrabberTwo 0)
      (CallFunction|Shoot))))

(fn ShowString
  (Rendering|SetVisibility (Variables|Default|GetCable) true true)
  (Rendering|SetVisibility (Variables|Default|GetCable1) true true))

(fn HideString
  (Rendering|SetVisibility (Variables|Default|GetCable) false true)
  (Rendering|SetVisibility (Variables|Default|GetCable1) false true))

(fn StringStrech
  (bind _grabbertwo (Variables|Default|GetGrabberTwo)
    (:then
      (bind _output_get (Variables|Default|SetStringRelativeLocation (Math|Vector|ProjectVectorontoVector (Math|Transform|InverseTransformLocation (Transformation|GetActorTransform) (Transformation|GetWorldLocation _grabbertwo)) (Math|Vector|GetRightVector (Variables|/Script/Engine.SceneComponent|GetRelativeRotation (Variables|Default|GetStaticMesh))))))
      (Variables|Default|SetStringCharge (Math|Vector|VectorLength (- (Variables|Default|GetStringRelativeLocation) (Variables|/Script/Engine.SceneComponent|GetRelativeLocation (Variables|Default|GetStringCollision)))))
      (if (and (< (Math|Vector|DotProduct (Math|Vector|Normalize (- (Variables|Default|GetStringRelativeLocation) (Variables|/Script/Engine.SceneComponent|GetRelativeLocation (Variables|Default|GetStringCollision)))) (Math|Vector|GetRightVector (Variables|/Script/Engine.SceneComponent|GetRelativeRotation (Variables|Default|GetStaticMesh)))) 0.0) (< (Math|Vector|VectorLength (- (Variables|Default|GetStringRelativeLocation) (Variables|/Script/Engine.SceneComponent|GetRelativeLocation (Variables|Default|GetStringCollision)))) 6e+01))
        (Transformation|SetRelativeLocation (Variables|Default|GetString) _output_get false false)
        (Variables|Default|SetCanEnchantArrow (>= (Math|Vector|VectorLength (- (Variables|Default|GetStringRelativeLocation) (Variables|/Script/Engine.SceneComponent|GetRelativeLocation (Variables|Default|GetStringCollision)))) 5e+01))))
    (:else)))

(fn ExecuteSkill
  (bind _arrow (Variables|Default|GetArrow)
    (:then
      (Default|EnchantArrow _arrow))
    (:else)))

(fn CanCast
  (return (Variables|Default|GetCanEnchantArrow)))