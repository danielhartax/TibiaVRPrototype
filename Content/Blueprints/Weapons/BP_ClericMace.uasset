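; BP_ClericMace is the cleric's mace weapon Blueprint, with a skill that heals the player.
; ExecuteSkill plays a heal sound at the mace's location and calls Heal on PlayerClass with a fixed amount.
; CanCast allows the skill only while the mace is higher than the player camera, so it works as a raise-overhead gesture.
; The event graph has no live logic, only disabled events and an unreached debug check for attachment to BP_PlayerFloatingHands.
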(event EventBeginPlay
  (|CallParentFunction) ; This node is disabled and will not be called.\nDrag off pins to build functionality.
)

(event Collision|EventActorBeginOverlap
  (params (OtherActor :type Actor%20Object%20Reference))
  (|CallParentFunction OtherActor) ; This node is disabled and will not be called.\nDrag off pins to build functionality.
)

(event EventTick
  (params (DeltaSeconds :type Float%20%28single-precision%29))
  (|CallParentFunction DeltaSeconds) ; This node is disabled and will not be called.\nDrag off pins to build functionality.
)

(fn ConstructionScript
  (|CallParentFunction))

(fn ExecuteSkill
  (Audio|PlaySoundatLocation "/Game/SFX/Weapons/Heal_cue.Heal_cue" (Transformation|GetActorLocation) "0, 0, 0" 1.0 1.0 0.0 0 0 0 0)
  (Default|Heal (Variables|Default|GetPlayerClass) 10))

(fn CanCast
  (return (< (.z (Camera|GetCameraLocation (Game|GetPlayerCameraManager 0))) (.z (Transformation|GetActorLocation self)))))