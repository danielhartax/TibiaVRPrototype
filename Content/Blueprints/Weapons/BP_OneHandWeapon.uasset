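; BP_OneHandWeapon is a one-handed weapon that deals dice-rolled melee damage to monsters.
; When its mesh begins overlapping a BP_Monster, it applies summed random rolls as damage, plays a hit sound and locks further hits until an overlap ends.
; A CastSkill event runs ExecuteSkill after a CanCast check, but both are placeholders: the check always passes and the skill only prints a message.
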(event OnComponentBeginOverlap(StaticMesh)
  (params (OverlappedComponent :type Primitive%20Component%20Object%20Reference) (OtherActor :type Actor%20Object%20Reference) (OtherComp :type Primitive%20Component%20Object%20Reference) (OtherBodyIndex :type Integer) (bFromSweep :type Boolean) (SweepResult :type Hit%20Result%20Structure%20%28by%20ref%29))
  ;[1 1 1] Damage
  (if (Variables|Default|GetCanHit)
    (if (Class|GameplayStatics|ObjectIsA OtherActor "/Game/Blueprints/Monsters/BP_Monster.BP_Monster_C")
      (Game|Damage|ApplyDamage OtherActor (Math|Conversions|ToFloat(Integer) (CallFunction|RollDice (Variables|Default|GetDamageDice) (Variables|Default|GetDiceQuantity))) 0 0)
      (Audio|PlaySoundatLocation "/Game/SFX/Weapons/Hammer.Hammer" (Transformation|GetWorldLocation (Variables|Default|GetStaticMesh)) "0, 0, 0" 1.0 1.0 0.0 0 0 0 0)
      (Variables|Default|SetCanHit false))))

(event OnComponentEndOverlap(StaticMesh)
  (params (OverlappedComponent :type Primitive%20Component%20Object%20Reference) (OtherActor :type Actor%20Object%20Reference) (OtherComp :type Primitive%20Component%20Object%20Reference) (OtherBodyIndex :type Integer))
  ;[1 1 1] Damage
  (Variables|Default|SetCanHit true))

(event EventBeginPlay
  (|CallParentFunction) ; This node is disabled and will not be called.\nDrag off pins to build functionality.
)

(event Collision|EventActorBeginOverlap
  (params (OtherActor :type Actor%20Object%20Reference))
  (|CallParentFunction OtherActor) ; This node is disabled and will not be called.\nDrag off pins to build functionality.
)

(event EventTick
  (params (DeltaSeconds :type Float%20%28single-precision%29))
  (|CallParentFunction DeltaSeconds) ; This node is disabled and will not be called.\nDrag off pins to build functionality.
)

(event EventCastSkill
  (bind _cancast (CallFunction|CanCast))
  (if _cancast
    (CallFunction|ExecuteSkill)))

(fn ConstructionScript
  (|CallParentFunction))

(fn RollDice
  (params (Dice :type Integer) (Quantity :type Integer))
  (for _index (range 0 Quantity)
    (LocalVariables|SetTempResult (+ (LocalVariables|GetTempResult) (Math|Random|RandomInteger Dice))))
  (return (LocalVariables|GetTempResult)))

(fn CanCast
  (return true))

(fn ExecuteSkill
  (Development|PrintString "Executou a magia" true true "(R=1.000000,G=0.420393,B=0.208745,A=1.000000)"))