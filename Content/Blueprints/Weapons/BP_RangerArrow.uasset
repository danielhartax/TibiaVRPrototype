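; BP_RangerArrow is an arrow projectile actor, named for the Ranger, that is launched by a Shoot event and halts on overlap.
; Shoot sets the projectile movement's initial and max speed to the given velocity, fires it along local X and enables query-only box collision.
; Any overlap on the box stops and deactivates movement and disables collision, with no damage or attachment logic in this graph.
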(event OnComponentBeginOverlap(BoxCollision)
  (params (OverlappedComponent :type Primitive%20Component%20Object%20Reference) (OtherActor :type Actor%20Object%20Reference) (OtherComp :type Primitive%20Component%20Object%20Reference) (OtherBodyIndex :type Integer) (bFromSweep :type Boolean) (SweepResult :type Hit%20Result%20Structure%20%28by%20ref%29))
  (bind _projectilemovement (Variables|Default|GetProjectileMovement))
  (Components|Movement|StopMovementImmediately _projectilemovement)
  (Components|Activation|SetActive _projectilemovement false false)
  (Collision|SetCollisionEnabled (Variables|Default|GetBoxCollision) "NoCollision"))

(event Custom|Shoot
  (params (Velocity :type Float%20%28double-precision%29))
  (bind _projectilemovement (Variables|Default|GetProjectileMovement))
  (bind _output_get (Variables|/Script/Engine.ProjectileMovementComponent|SetInitialSpeed _projectilemovement Velocity))
  (bind _output_get_2 (Variables|/Script/Engine.ProjectileMovementComponent|SetMaxSpeed _projectilemovement _output_get))
  (Game|Components|ProjectileMovement|SetVelocityinLocalSpace _projectilemovement (Math|Vector|MakeVector _output_get_2 0.0 0.0))
  (Components|Activation|SetActive _projectilemovement true false)
  (Collision|SetCollisionEnabled (Variables|Default|GetBoxCollision) "QueryOnly"))

(event EventBeginPlay)

(event Collision|EventActorBeginOverlap
  (params (OtherActor :type Actor%20Object%20Reference)))

(event EventTick
  (params (DeltaSeconds :type Float%20%28single-precision%29)))

(fn ConstructionScript)