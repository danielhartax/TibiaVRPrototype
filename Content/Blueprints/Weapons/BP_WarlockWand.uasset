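; BP_WarlockWand is a VR wand weapon that can cast only while the player is concentrating.
; Concentration turns on when a component attached to a motion controller enters the wand's Sphere while GrabberOne is valid, and off when one leaves.
; CanCast returns that concentration flag.
; ExecuteSkill is a placeholder that only prints a red "FLAMES" debug string.
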(event OnComponentBeginOverlap(Sphere)
  (params (OverlappedComponent :type Primitive%20Component%20Object%20Reference) (OtherActor :type Actor%20Object%20Reference) (OtherComp :type Primitive%20Component%20Object%20Reference) (OtherBodyIndex :type Integer) (bFromSweep :type Boolean) (SweepResult :type Hit%20Result%20Structure%20%28by%20ref%29))
  ;[1 1 1] Liga e desliga a concentração
  (Utilities|IsValid (Variables|Default|GetGrabberOne)
    (:Is%20Valid
      (Utilities|Casting|CastToMotionControllerComponent (Transformation|GetAttachParent OtherComp))
      (Variables|Default|SetIsConcentranting true))))

(event OnComponentEndOverlap(Sphere)
  (params (OverlappedComponent :type Primitive%20Component%20Object%20Reference) (OtherActor :type Actor%20Object%20Reference) (OtherComp :type Primitive%20Component%20Object%20Reference) (OtherBodyIndex :type Integer))
  ;[1 1 1] Liga e desliga a concentração
  (Utilities|Casting|CastToMotionControllerComponent (Transformation|GetAttachParent OtherComp))
  (Variables|Default|SetIsConcentranting false))

(event EventBeginPlay
  (|CallParentFunction) ; This node is disabled and will not be called.\nDrag off pins to build functionality.
)

(event Collision|EventActorBeginOverlap
  (params (OtherActor :type Actor%20Object%20Reference))
  (|CallParentFunction OtherActor) ; This node is disabled and will not be called.\nDrag off pins to build functionality.
)

(event EventTick
  (params (DeltaSeconds :type Float%20%28single-precision%29))
  (|CallParentFunction DeltaSeconds) ; This node is disabled and will not be called.\nDrag off pins to build functionality.
)

(fn ConstructionScript
  (|CallParentFunction))

(fn CanCast
  (return (Variables|Default|GetIsConcentranting)))

(fn ExecuteSkill
  (Development|PrintString "FLAMES" true true "(R=1.000000,G=0.010197,B=0.030093,A=1.000000)"))