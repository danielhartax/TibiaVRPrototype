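; Grabbable physics actor in the Weapons folder that can be held by one or two hands.
; Grab disables mesh physics, attaches the actor to the grabbing component and records it as GrabberOne or GrabberTwo.
; While both are valid, Tick snaps the actor to GrabberOne and rotates it to look at GrabberTwo.
; Drop clears that grabber, then reattaches to the remaining one or re-enables physics when none remain.
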(event EventBeginPlay)

(event Collision|EventActorBeginOverlap
  (params (OtherActor :type Actor%20Object%20Reference)))

(event EventTick
  (params (DeltaSeconds :type Float%20%28single-precision%29))
  (CallFunction|AdjustRotationifIsHeldwithTwoHands))

(event EventGrab
  (params (AttatchTo :type Scene%20Component%20Object%20Reference))
  ;[1 1 1] Grab
  (Physics|SetSimulatePhysics (Variables|Default|GetStaticMesh) false)
  (Transformation|AttachComponentToComponent (Variables|Transformation|GetRootComponent) AttatchTo "" "KeepWorld" "KeepWorld" "KeepWorld" false)
  (Utilities|IsValid (Variables|Default|GetGrabberOne)
    (:Is%20Valid
      (Variables|Default|SetGrabberTwo AttatchTo))
    (:Is%20Not%20Valid
      (Variables|Default|SetGrabberOne AttatchTo))))

(event EventDrop
  (params (Grabber :type Scene%20Component%20Object%20Reference))
  (bind _grabberone (Variables|Default|GetGrabberOne))
  (bind _nohandholding (CallFunction|CheckHandHolding Grabber))
  (Physics|SetSimulatePhysics (Variables|Default|GetStaticMesh) _nohandholding)
  (Transformation|DetachFromActor "KeepWorld" "KeepWorld" "KeepWorld")
  (if (not _nohandholding)
    (if (Utilities|IsValid _grabberone)
      (Transformation|AttachComponentToComponent (Variables|Transformation|GetRootComponent) _grabberone "" "KeepWorld" "KeepWorld" "KeepWorld" false)
      (else
        (Transformation|AttachComponentToComponent (Variables|Transformation|GetRootComponent) (Variables|Default|GetGrabberTwo) "" "KeepWorld" "KeepWorld" "KeepWorld" false)))))

(fn ConstructionScript)

(fn AdjustRotationifIsHeldwithTwoHands
  (bind _grabberone (Variables|Default|GetGrabberOne))
  (bind _grabbertwo (Variables|Default|GetGrabberTwo))
  (bind _returnvalue (Transformation|GetWorldLocation _grabberone))
  (Utilities|IsValid _grabberone
    (:Is%20Valid
      (Utilities|IsValid _grabbertwo
        (:Is%20Valid
          (Transformation|SetActorLocation _returnvalue false false)
          (Transformation|SetActorRotation (Math|Rotator|FindLookatRotation _returnvalue (Transformation|GetWorldLocation _grabbertwo))))))))

(fn CheckHandHolding
  (params (Grabber :type Scene%20Component%20Object%20Reference))
  (if (== (Variables|Default|GetGrabberOne) Grabber)
    (Variables|Default|SetGrabberOne 0))
  (if (== (Variables|Default|GetGrabberTwo) Grabber)
    (Variables|Default|SetGrabberTwo 0))
  (return (not (or (Utilities|IsValid (Variables|Default|GetGrabberOne)) (Utilities|IsValid (Variables|Default|GetGrabberTwo))))))