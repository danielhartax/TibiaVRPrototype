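; BP_BarbarianAxe is a weapon Blueprint for the barbarian's axe, with a castable skill.
; CanCast allows the skill only when both GrabberOne and GrabberTwo are valid, which suggests a two-handed grip requirement.
; ExecuteSkill is a placeholder that only prints a red debug message, and the default event and construction graphs add no logic of their own.
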(event EventBeginPlay
  (|CallParentFunction) ; This node is disabled and will not be called.\nDrag off pins to build functionality.
)

(event Collision|EventActorBeginOverlap
  (params (OtherActor :type Actor%20Object%20Reference))
  (|CallParentFunction OtherActor) ; This node is disabled and will not be called.\nDrag off pins to build functionality.
)

(event EventTick
  (params (DeltaSeconds :type Float%20%28single-precision%29))
  (|CallParentFunction DeltaSeconds) ; This node is disabled and will not be called.\nDrag off pins to build functionality.
)

(fn ConstructionScript
  (|CallParentFunction))

(fn CanCast
  (return (and (Utilities|IsValid (Variables|Default|GetGrabberOne)) (Utilities|IsValid (Variables|Default|GetGrabberTwo)))))

(fn ExecuteSkill
  (Development|PrintString "Barbaro castou" true true "(R=1.000000,G=0.000000,B=0.116823,A=1.000000)"))