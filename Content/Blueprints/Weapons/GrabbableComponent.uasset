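; Weapon component that makes its owning actor grabbable with one or two hands.
; Grab disables DamageDealerMesh physics, attaches the owner to the grabber and records up to two grabbers.
; Each tick with both held, the owner snaps to GrabberOne and aims at GrabberTwo.
; Drop always detaches, restoring physics once no grabber remains; reattachment to a remaining hand is left unwired.
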(event EventBeginPlay)

(event EventTick
  (params (DeltaSeconds :type Float%20%28single-precision%29))
  (CallFunction|AdjustRotationifIsHeldwithTwoHands))

(event EventGrab
  (params (AttatchTo :type Scene%20Component%20Object%20Reference))
  (bind _returnvalue (Components|GetOwner))
  (bind _rootcomponent (Variables|/Script/Engine.Actor|GetRootComponent _returnvalue))
  ;[1 1 1] Grab
  (Development|PrintString (Utilities|GetDisplayName AttatchTo))
  (Physics|SetSimulatePhysics (Variables|Components|GetDamageDealerMesh) false)
  (Transformation|AttachComponentToComponent _rootcomponent AttatchTo "" "KeepWorld" "KeepWorld" "KeepWorld" false)
  (Development|PrintString (Utilities|GetDisplayName _rootcomponent))
  (Utilities|IsValid (Variables|Default|GetGrabberOne)
    (:Is%20Valid
      (Variables|Default|SetGrabberTwo AttatchTo))
    (:Is%20Not%20Valid
      (Variables|Default|SetGrabberOne AttatchTo))))

(event EventDrop
  (params (Grabber :type Scene%20Component%20Object%20Reference))
  (bind _returnvalue (Components|GetOwner))
  (Development|PrintString (Utilities|GetDisplayName Grabber))
  (bind _nohandholding (CallFunction|CheckHandHolding Grabber))
  (Physics|SetSimulatePhysics (Variables|Components|GetDamageDealerMesh) _nohandholding)
  (Development|PrintString (Utilities|GetDisplayName (Variables|/Script/Engine.Actor|GetRootComponent _returnvalue)))
  (Transformation|DetachFromActor _returnvalue "KeepWorld" "KeepWorld" "KeepWorld")
  (if (not _nohandholding)
    (if (Utilities|IsValid (Variables|Default|GetGrabberOne))
      _)))

(fn CheckHandHolding
  (params (Grabber :type Scene%20Component%20Object%20Reference))
  (if (== (Variables|Default|GetGrabberOne) Grabber)
    (Variables|Default|SetGrabberOne 0))
  (if (== (Variables|Default|GetGrabberTwo) Grabber)
    (Variables|Default|SetGrabberTwo 0))
  (return (not (or (Utilities|IsValid (Variables|Default|GetGrabberOne)) (Utilities|IsValid (Variables|Default|GetGrabberTwo))))))

(fn AdjustRotationifIsHeldwithTwoHands
  (bind _returnvalue (Components|GetOwner))
  (bind _grabberone (Variables|Default|GetGrabberOne))
  (bind _grabbertwo (Variables|Default|GetGrabberTwo))
  (bind _returnvalue_2 (Transformation|GetWorldLocation _grabberone))
  (Utilities|IsValid _grabberone
    (:Is%20Valid
      (Utilities|IsValid _grabbertwo
        (:Is%20Valid
          (Transformation|SetActorLocation _returnvalue _returnvalue_2 false false)
          (Transformation|SetActorRotation _returnvalue (Math|Rotator|FindLookatRotation _returnvalue_2 (Transformation|GetWorldLocation _grabbertwo))))))))